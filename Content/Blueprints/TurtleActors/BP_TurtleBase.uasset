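; BP_TurtleBase is a turtle character base with custom events for moving between its start location and a TargetPoint actor.
; GoDestinat and Gostar each issue an AI MoveToLocation, then set a time-expired flag after a delay; Gostar also flips the mesh yaw.
; The setup and flag-based ping-pong logic that would alternate them is disconnected, leaving BeginPlay and Tick empty, so this Blueprint never starts the movement itself.
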(event `Gostar`
  (bind _mesh (`self.Mesh`))
  (`SceneComponent.K2_AddWorldRotation` _mesh (struct :`Yaw` 180.0) false false)
  (`AIController.MoveToLocation` (`AIBlueprintHelperLibrary.GetAIController` null) (`self.StartLoc`) -1.0 true true false true null true)
  (set `CharacterMovementComponent.bOrientRotationToMovement` false (`self.CharacterMovement`))
  (`KismetSystemLibrary.Delay` 1.0)
  (set `self.Timeexpiried` true)
  (`KismetSystemLibrary.Delay` (`self.GetActorTickInterval`))
  (`SceneComponent.K2_AddWorldRotation` _mesh (struct :`Yaw` 180.0) false false))

(event `GoDestinat`
  (`AIController.MoveToLocation` (`AIBlueprintHelperLibrary.GetAIController` null) (`self.K2_GetActorLocation` (`self.destination`)) -1.0 true true false true null true)
  (`KismetSystemLibrary.Delay` 2.0)
  (set `self.Timeexpiried` true))

(event `self.ReceiveBeginPlay`)

(event `self.ReceiveTick`
  (params (DeltaSeconds :type "Float (single-precision)")))

(fn `UserConstructionScript`)