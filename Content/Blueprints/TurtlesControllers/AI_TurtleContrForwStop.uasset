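; AI controller that walks a turtle pawn toward TargetToMove in a stop-and-go rhythm.
; Tick reissues MoveToLocation while in the moving phase, and destroys both pawn and controller once the goal is reached.
; Two delay-driven events set a time-expired flag, which Tick uses with phase booleans to alternate roughly one second of movement with a half-second stop.
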(event `Gostar`
  (`self.StopMovement`)
  (`KismetSystemLibrary.Delay` 0.5)
  (set `self.Timeexpiried` true))

(event `GoDestinat`
  (`KismetSystemLibrary.Delay` 1.0)
  (set `self.Timeexpiried` true))

(event `self.ReceiveBeginPlay`
  (`self.GoDestinat`)
  (set `self.GoDest` true)
  (set `self.GoStartloc` false))

(event `self.ReceiveTick`
  (params (DeltaSeconds :type "Float (single-precision)"))
  (bind _timeexpiried (`self.Timeexpiried`))
  (if (`self.GoDest`)
    (bind _returnvalue (`self.MoveToLocation` (`self.K2_GetActorLocation` (`self.TargetToMove`)) -1.0 true true false true null))
    (switch `EPathFollowingRequestResult` _returnvalue
      (:`AlreadyAtGoal`
        (`self.K2_DestroyActor` (`self.K2_GetPawn`))
        (`self.K2_DestroyActor`))
      (:`RequestSuccessful`
        (if _timeexpiried
          (`self.Gostar`)
          (set `self.Timeexpiried` false)
          (set `self.GoStartloc` true)
          (set `self.GoDest` false))))
    (elif (`self.GoStartloc`)
      (if _timeexpiried
        (set `self.Timeexpiried` false)
        (`self.GoDestinat`)
        (set `self.GoStartloc` false)
        (set `self.GoDest` true)))))

(fn `UserConstructionScript`)