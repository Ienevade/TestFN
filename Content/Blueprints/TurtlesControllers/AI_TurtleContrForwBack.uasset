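; AI controller that shuttles a BP_TurtleBase pawn back and forth between its spawn location and a TargetPoint found in the level.
; Tick alternates the two MoveToLocation legs using boolean flags, switched by fixed delays rather than arrival.
; The return leg flips the mesh 180 degrees, disables orient-to-movement (never restored), and flips the mesh back as the next outbound leg starts.
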(event `Gostar`
  (bind _asbp_turtle_base (cast `/Game/Blueprints/TurtleActors/BP_TurtleBase` (`self.K2_GetPawn`)))
  (bind _mesh (`Character.Mesh` _asbp_turtle_base))
  (`SceneComponent.K2_AddWorldRotation` _mesh (struct :`Yaw` 180.0) false false)
  (`self.MoveToLocation` (`self.StartLoc`) -1.0 true true false true null)
  (set `CharacterMovementComponent.bOrientRotationToMovement` false (`Character.CharacterMovement` _asbp_turtle_base))
  (`KismetSystemLibrary.Delay` 1.0)
  (set `self.Timeexpiried` true)
  (`KismetSystemLibrary.Delay` (`self.GetActorTickInterval`))
  (`SceneComponent.K2_AddWorldRotation` _mesh (struct :`Yaw` 180.0) false false))

(event `GoDestinat`
  (`self.MoveToLocation` (`self.K2_GetActorLocation` (`self.destination`)) -1.0 true true false true null)
  (`KismetSystemLibrary.Delay` 2.0)
  (set `self.Timeexpiried` true))

(event `self.ReceiveBeginPlay`
  (bind _returnvalue (`GameplayStatics.GetActorOfClass` "/Script/Engine.TargetPoint"))
  (set `self.destination` _returnvalue)
  (set `self.StartLoc` (`self.K2_GetActorLocation` (`self.K2_GetPawn`)))
  (`self.GoDestinat`)
  (set `self.GoDest` true)
  (set `self.GoStartloc` false))

(event `self.ReceiveTick`
  (params (DeltaSeconds :type "Float (single-precision)"))
  (bind _timeexpiried (`self.Timeexpiried`))
  (if (`self.GoDest`)
    (if _timeexpiried
      (`self.Gostar`)
      (set `self.Timeexpiried` false)
      (set `self.GoStartloc` true)
      (set `self.GoDest` false))
    (elif (`self.GoStartloc`)
      (if _timeexpiried
        (set `self.Timeexpiried` false)
        (`self.GoDestinat`)
        (set `self.GoStartloc` false)
        (set `self.GoDest` true)))))

(fn `UserConstructionScript`)